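; BP_Door is a double door that opens when a BP_Character overlaps it, playing a 2D opening sound.
; The overlap sets a flag that makes Tick yaw two InvisibleCube components in opposite directions.
; Both rotation steps scale with the angle between the first cube's right vector and the root's forward vector, so the swing eases out as they align.
; No logic closes the door.
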(event `self.ReceiveActorBeginOverlap`
  (params (OtherActor :type "Actor Object Reference"))
  (cast `/Game/Blueprints/BP_Character` OtherActor)
  (`GameplayStatics.PlaySound2D` "/Game/audio/DoorOpening.DoorOpening" 1.0 1.0 0.0 null null)
  (set `self.ShouldOpen` true))

(event `self.ReceiveTick`
  (params (DeltaSeconds :type "Float (single-precision)"))
  (bind _returnvalue (* DeltaSeconds (`KismetMathLibrary.DegAcos` (`KismetMathLibrary.Dot_VectorVector` (`SceneComponent.GetRightVector` (`self.InvisibleCube`)) (`SceneComponent.GetForwardVector` (`self.DefaultSceneRoot`)))) (`self.Speed`)))
  (if (`self.ShouldOpen`)
    (`SceneComponent.K2_AddLocalRotation` (`self.InvisibleCube`) (`KismetMathLibrary.MakeRotator` 0.0 0.0 _returnvalue) false false)
    (`SceneComponent.K2_AddLocalRotation` (`self.InvisibleCube1`) (`KismetMathLibrary.MakeRotator` 0.0 0.0 (* _returnvalue -1.0)) false false)))

(fn `UserConstructionScript`)