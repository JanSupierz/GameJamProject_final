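; Two-player co-op character in which both players, controlled from one Blueprint, carry a table with a pot on it.
; Axis inputs move each player unless sliding, and button presses raise individual hands, which sink back down every tick.
; Tick centers the camera socket between players, derives the table's position and rotation from the four hands, and slides the pot when tilt exceeds a margin.
; It also creates the HUD and tutorial widgets, removing the tutorial once the game starts.
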(event `self.ReceiveTick`
  (params (DeltaSeconds :type "Float (single-precision)"))
  (bind _table (`self.Table`))
  (bind _pot (`self.Pot`))
  (bind _pot_2 (`self.Pot`))
  (bind _returnvalue (`SceneComponent.GetRightVector` (`self.Table`)))
  (bind _returnvalue_2 (`SceneComponent.GetForwardVector` (`self.Table`)))
  (bind _returnvalue_3 (`KismetMathLibrary.Dot_VectorVector` _returnvalue_2 (0.0 0.0 1.0)))
  (bind _returnvalue_4 (`KismetMathLibrary.Dot_VectorVector` _returnvalue (0.0 0.0 1.0)))
  (bind _returnvalue_5 (`KismetMathLibrary.Normal` (- (`SceneComponent.K2_GetComponentLocation` (`self.RightHand`)) (`SceneComponent.K2_GetComponentLocation` (`self.RightHand1`)))))
  (bind _returnvalue_6 (`KismetMathLibrary.Normal` (- (`SceneComponent.K2_GetComponentLocation` (`self.RightHand`)) (`SceneComponent.K2_GetComponentLocation` (`self.LeftHand`)))))
  (bind _returnvalue_7 (`KismetMathLibrary.Normal` (- (`SceneComponent.K2_GetComponentLocation` (`self.RightHand1`)) (`SceneComponent.K2_GetComponentLocation` (`self.LeftHand1`)))))
  (bind _returnvalue_8 (`KismetMathLibrary.DegAcos` (`KismetMathLibrary.Dot_VectorVector` _returnvalue_6 (`SceneComponent.GetRightVector` (`self.CameraSocket`)))))
  (bind _returnvalue_9 (`KismetMathLibrary.DegAcos` (`KismetMathLibrary.Dot_VectorVector` _returnvalue_7 (`SceneComponent.GetRightVector` (`self.CameraSocket`)))))
  (bind _returnvalue_10 (+ (`KismetMathLibrary.DegAcos` (`KismetMathLibrary.Dot_VectorVector` _returnvalue_5 (`SceneComponent.GetRightVector` (`self.CameraSocket`)))) 90.0))
  ;[1 1 1] Getting weak
  (`|ExecutionSequence`
    (:`then_0`
      (bind _asbp_my_game_mode (cast `/Game/Blueprints/BP_MyGameMode` (`GameplayStatics.GetGameMode`)))
      (if (`/Game/Blueprints/BP_MyGameMode.hasGameStarted` _asbp_my_game_mode)
        (bind _tutorialhudrer (`self.TutorialHUDRer`)
          (:`then`
            (`Widget.RemoveFromParent` _tutorialhudrer))
          (:`else`))))
    (:`then_1`
      (`self.LowerHands` (`self.RightHand`) DeltaSeconds)
      (`self.LowerHands` (`self.LeftHand`) DeltaSeconds)
      (`self.LowerHands` (`self.LeftHand1`) DeltaSeconds)
      (`self.LowerHands` (`self.RightHand1`) DeltaSeconds)
      (`SceneComponent.K2_SetWorldLocation` (`self.CameraSocket`) (+ (/ (+ (`SceneComponent.K2_GetComponentLocation` (`self.Player1`)) (`SceneComponent.K2_GetComponentLocation` (`self.Player2`))) (2.0 2.0 2.0)) (0.0 0.0 100.0)) false false)
      (if (> (.z _returnvalue_6) 0.0)
        (set `self.AngleX_1` _returnvalue_8)
        (else
          (set `self.AngleX_1` (* _returnvalue_8 -1.0))))
      (if (> (.z _returnvalue_7) 0.0)
        (set `self.AngleX_2` _returnvalue_9)
        (else
          (set `self.AngleX_2` (* _returnvalue_9 -1.0))))
      (set `self.AngleY_1` (+ (`KismetMathLibrary.DegAcos` (`KismetMathLibrary.Dot_VectorVector` (`KismetMathLibrary.Normal` (- (`SceneComponent.K2_GetComponentLocation` (`self.LeftHand1`)) (`SceneComponent.K2_GetComponentLocation` (`self.LeftHand`)))) (0.0 0.0 1.0))) -90.0))
      (set `self.AngleY_2` (+ (`KismetMathLibrary.DegAcos` (`KismetMathLibrary.Dot_VectorVector` (`KismetMathLibrary.Normal` (- (`SceneComponent.K2_GetComponentLocation` (`self.RightHand1`)) (`SceneComponent.K2_GetComponentLocation` (`self.RightHand`)))) (0.0 0.0 1.0))) -90.0))
      (set `self.AngleX` (/ (+ (`self.AngleX_1`) (`self.AngleX_2`)) 2.0))
      (set `self.AngleY` (/ (+ (`self.AngleY_1`) (`self.AngleY_2`)) 2.0))
      (if (> (.y _returnvalue_5) 0.0)
        (`SceneComponent.K2_SetRelativeRotation` _table (`KismetMathLibrary.MakeRotator` (`self.AngleX`) (`self.AngleY`) _returnvalue_10) false false)
        (else
          (`SceneComponent.K2_SetRelativeRotation` _table (`KismetMathLibrary.MakeRotator` (`self.AngleX`) (`self.AngleY`) _returnvalue_10) false false)))
      (`SceneComponent.K2_SetWorldLocation` (`self.Table`) (/ (+ (`SceneComponent.K2_GetComponentLocation` (`self.RightHand`)) (`SceneComponent.K2_GetComponentLocation` (`self.LeftHand`)) (`SceneComponent.K2_GetComponentLocation` (`self.RightHand1`)) (`SceneComponent.K2_GetComponentLocation` (`self.LeftHand1`))) (`self.divider`)) false false)
      (if (> (`KismetMathLibrary.Abs` _returnvalue_4) (`self.SlidingMargin`))
        (`SceneComponent.K2_SetWorldLocation` _pot (- (`SceneComponent.K2_GetComponentLocation` _pot) (* _returnvalue_4 _returnvalue)) false false))
      (if (> (`KismetMathLibrary.Abs` _returnvalue_3) (`self.SlidingMargin`))
        (`SceneComponent.K2_SetWorldLocation` _pot_2 (- (`SceneComponent.K2_GetComponentLocation` _pot_2) (* _returnvalue_3 _returnvalue_2)) false false)))))

(event `InputAxis|ForwardMovementPlayer1`
  (params (AxisValue :type "Float (single-precision)"))
  ;[1 1 1] Movement player 1
  (`self.MovePlayer` AxisValue (`self.Player1`) (`self.IsSlidingPlayer1`)))

(event `InputAxis|ForwardMovementPlayer2`
  (params (AxisValue :type "Float (single-precision)"))
  ;[1 1 1] Movement player 2
  (`self.MovePlayer` AxisValue (`self.Player2`) (`self.IsSlidingPlayer2`)))

(event `self.ReceiveBeginPlay`
  ;[1 1 1] Widget
  (bind _returnvalue (`|CreateWidget` "/Game/Blueprints/BP_HUD.BP_HUD_C"))
  (`UserWidget.AddToViewport` _returnvalue 0)
  (bind _returnvalue_2 (`|CreateWidget` "/Game/Blueprints/BP_TutorialHUD.BP_TutorialHUD_C"))
  (bind _output_get (set `self.TutorialHUDRer` _returnvalue_2))
  (`UserWidget.AddToViewport` _output_get 0))

(event `InputAxis|Rotate`
  (params (AxisValue :type "Float (single-precision)")))

(event `InputAction|LeftHandPlayer1`
  (params (Key :type "Key Structure"))
  ;[1 1 1] Player 1 hands
  (:`Pressed`
    (`SceneComponent.K2_AddLocalOffset` (`self.LeftHand`) (`KismetMathLibrary.MakeVector` 0.0 0.0 (`self.handOffset`)) false false)))

(event `InputAction|LeftHandPlayer2`
  (params (Key :type "Key Structure"))
  ;[1 1 1] Player 2 hands
  (:`Pressed`
    (`SceneComponent.K2_AddLocalOffset` (`self.LeftHand1`) (`KismetMathLibrary.MakeVector` 0.0 0.0 (`self.handOffset`)) false false)))

(event `InputAction|RightHandPlayer1`
  (params (Key :type "Key Structure"))
  ;[1 1 1] Player 1 hands
  (:`Pressed`
    (`SceneComponent.K2_AddLocalOffset` (`self.RightHand`) (`KismetMathLibrary.MakeVector` 0.0 0.0 (`self.handOffset`)) false false)))

(event `InputAction|RightHandPlayer2`
  (params (Key :type "Key Structure"))
  ;[1 1 1] Player 2 hands
  (:`Pressed`
    (`SceneComponent.K2_AddLocalOffset` (`self.RightHand1`) (`KismetMathLibrary.MakeVector` 0.0 0.0 (`self.handOffset`)) false false)))

(fn `LowerHands`
  (params (Hand :type "StaticMeshComponent Object Reference") (deltaTime :type "Float (double-precision)"))
  (bind (_relativelocation_x _relativelocation_y _relativelocation_z) (`KismetMathLibrary.BreakVector` (`SceneComponent.RelativeLocation` Hand)))
  (`SceneComponent.K2_SetRelativeLocation` Hand (`KismetMathLibrary.MakeVector` _relativelocation_x _relativelocation_y (`KismetMathLibrary.FClamp` (- _relativelocation_z (* (`self.heightDecay`) deltaTime)) (`self.minHeight`) (`self.maxHeight`))) false false))

(fn `MovePlayer`
  (params (DeltaLocation_Y :type "Float (double-precision)") (Player :type "SceneComponent Object Reference") (IsSliding :type Boolean))
  (if (not IsSliding)
    (`SceneComponent.K2_SetWorldLocation` Player (+ (`SceneComponent.K2_GetComponentLocation` Player) (* (`self.MoveDirection`) DeltaLocation_Y)) false false)))

(fn `UserConstructionScript`)