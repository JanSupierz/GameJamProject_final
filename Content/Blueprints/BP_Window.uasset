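; BP_Window is a two-pane window that swings open once, when the character first overlaps it, and pushes that character's pot.
; BeginPlay derives each pane's mirrored open rotation from SwingAngle, and Tick lerps the panes toward open or closed by DeltaSeconds times OpenSpeed.
; Opening plays a wind sound, shows Niagara and calls MovePot every tick.
; Ending the overlap closes it and hides the effect.
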(event `self.ReceiveBeginPlay`
  (bind _rightpart (`self.rightPart`))
  (bind (_returnvalue_roll _returnvalue_pitch _returnvalue_yaw) (`KismetMathLibrary.BreakRotator` (`SceneComponent.K2_GetComponentRotation` (`self.leftPart`))))
  (bind (_returnvalue_roll_2 _returnvalue_pitch_2 _returnvalue_yaw_2) (`KismetMathLibrary.BreakRotator` (`SceneComponent.K2_GetComponentRotation` _rightpart)))
  (`|ExecutionSequence`
    (:`then_0`
      (set `self.rightPartEndRotation` (`KismetMathLibrary.MakeRotator` _returnvalue_roll_2 _returnvalue_pitch_2 (+ _returnvalue_yaw_2 (`self.swingAngle`))))
      (set `self.rightPartStartRotation` (`SceneComponent.K2_GetComponentRotation` _rightpart)))
    (:`then_1`
      (set `self.leftPartEndRotation` (`KismetMathLibrary.MakeRotator` _returnvalue_roll _returnvalue_pitch (- _returnvalue_yaw (`self.swingAngle`))))
      (set `self.leftPartStartRotation` (`SceneComponent.K2_GetComponentRotation` (`self.leftPart`))))))

(event `self.ReceiveTick`
  (params (DeltaSeconds :type "Float (single-precision)"))
  (bind _rightpart (`self.rightPart`))
  (bind (_rightpartendrotation_roll _rightpartendrotation_pitch _rightpartendrotation_yaw) (`KismetMathLibrary.BreakRotator` (`self.rightPartEndRotation`)))
  (bind _leftpart (`self.leftPart`))
  (bind _leftpart_2 (`self.leftPart`))
  (bind (_leftpartendrotation_roll _leftpartendrotation_pitch _leftpartendrotation_yaw) (`KismetMathLibrary.BreakRotator` (`self.leftPartEndRotation`)))
  (bind _rightpart_2 (`self.rightPart`))
  (bind (_returnvalue_roll _returnvalue_pitch _returnvalue_yaw) (`KismetMathLibrary.BreakRotator` (`SceneComponent.K2_GetComponentRotation` (`self.rightPart`))))
  (bind (_returnvalue_roll_2 _returnvalue_pitch_2 _returnvalue_yaw_2) (`KismetMathLibrary.BreakRotator` (`SceneComponent.K2_GetComponentRotation` (`self.leftPart`))))
  (`|ExecutionSequence`
    (:`then_0`
      (if true
        (if (and (`self.open`) (< _returnvalue_yaw _rightpartendrotation_yaw))
          (`SceneComponent.K2_SetWorldRotation` _rightpart_2 (`KismetMathLibrary.RLerp` (`SceneComponent.K2_GetComponentRotation` _rightpart_2) (`self.rightPartEndRotation`) (* DeltaSeconds (`self.openSpeed`))) false false)
          (else
            (`SceneComponent.K2_SetWorldRotation` _rightpart (`KismetMathLibrary.RLerp` (`SceneComponent.K2_GetComponentRotation` _rightpart) (`self.rightPartStartRotation`) (* (`self.openSpeed`) DeltaSeconds)) false false)))))
    (:`then_1`
      (if (and (`self.open`) (> _returnvalue_yaw_2 _leftpartendrotation_yaw))
        (`SceneComponent.K2_SetWorldRotation` _leftpart (`KismetMathLibrary.RLerp` (`SceneComponent.K2_GetComponentRotation` _leftpart) (`self.leftPartEndRotation`) (* DeltaSeconds (`self.openSpeed`))) false false)
        (else
          (`SceneComponent.K2_SetWorldRotation` _leftpart_2 (`KismetMathLibrary.RLerp` (`SceneComponent.K2_GetComponentRotation` _leftpart_2) (`self.leftPartStartRotation`) (* (`self.openSpeed`) DeltaSeconds)) false false))))
    (:`then_2`
      (if (`self.open`)
        (bind _characterref (`self.characterRef`)
          (:`then`
            (`/Game/Blueprints/BP_Character.MovePot` _characterref (`self.PotMoveDirection`)))
          (:`else`))))))

(event `self.ReceiveActorBeginOverlap`
  (params (OtherActor :type "Actor Object Reference"))
  (if (not (`self.hasBeenOpenedBefore`))
    (bind _asbp_character (cast `/Game/Blueprints/BP_Character` OtherActor))
    (set `self.characterRef` _asbp_character)
    (if (not (`self.open`))
      (`GameplayStatics.PlaySound2D` "/Game/audio/WindSound.WindSound" 1.0 1.0 0.0 null null)
      (set `self.open` true)
      (set `self.hasBeenOpenedBefore` true)
      (`SceneComponent.SetHiddenInGame` (`self.Niagara`) false false))))

(event `self.ReceiveActorEndOverlap`
  (params (OtherActor :type "Actor Object Reference"))
  (cast `/Game/Blueprints/BP_Character` OtherActor)
  (if (`self.open`)
    (set `self.open` false)
    (`SceneComponent.SetHiddenInGame` (`self.Niagara`) true false)))

(fn `UserConstructionScript`)