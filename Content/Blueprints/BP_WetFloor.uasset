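; BP_WetFloor is a slippery floor hazard that takes movement control from a player and slides them along world +Y.
; Box overlap with BP_Character picks Player1 or Player2 by the floor's PlayerNumber, sets its CanPlayerNotMove flag and plays a slip sound.
; Tick calls the character's MovePlayer, scaled by SlideSpeed and delta time, while either flag is set.
; Ending overlap clears both players' flags; an older lerp-based slide remains unconnected.
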(event `self.ReceiveTick`
  (params (DeltaSeconds :type "Float (single-precision)"))
  (`self.playerRef`
    (:`then`
      (`self.characterRef`
        (:`then`
          (if (or (`/Game/Blueprints/BP_Character.CanPlayer1NotMove` (`self.characterRef`)) (`/Game/Blueprints/BP_Character.CanPlayer2NotMove` (`self.characterRef`)))
            (`/Game/Blueprints/BP_Character.MovePlayer` (`self.characterRef`) (* (`self.slideSpeed`) DeltaSeconds) (`self.playerRef`) false (0.0 1.0 0.0))))
        (:`else`)))
    (:`else`)))

(event `self.Box.OnComponentBeginOverlap`
  (params (OverlappedComponent :type "PrimitiveComponent Object Reference") (OtherActor :type "Actor Object Reference") (OtherComp :type "PrimitiveComponent Object Reference") (OtherBodyIndex :type Integer) (bFromSweep :type Boolean) (SweepResult :type "HitResult Structure (by ref)"))
  (bind _playernumber (`self.playerNumber`))
  (bind _asbp_character (cast `/Game/Blueprints/BP_Character` OtherActor))
  (set `self.characterRef` _asbp_character)
  (if (== _playernumber 1)
    (set `self.playerRef` (`/Game/Blueprints/BP_Character.Player1` (`self.characterRef`)))
    (set `/Game/Blueprints/BP_Character.CanPlayer1NotMove` true (`self.characterRef`))
    (`GameplayStatics.PlaySound2D` "/Game/audio/Slippery_Floor_Sound_Effect.Slippery_Floor_Sound_Effect" 1.0 1.0 0.0 null null :!label _label)
    (elif (== _playernumber 2)
      (set `self.playerRef` (`/Game/Blueprints/BP_Character.Player2` (`self.characterRef`)))
      (set `/Game/Blueprints/BP_Character.CanPlayer2NotMove` true (`self.characterRef`))
      (goto _label))))

(event `self.Box.OnComponentEndOverlap`
  (params (OverlappedComponent :type "PrimitiveComponent Object Reference") (OtherActor :type "Actor Object Reference") (OtherComp :type "PrimitiveComponent Object Reference") (OtherBodyIndex :type Integer))
  (bind _characterref (`self.characterRef`)
    (:`then`
      (set `/Game/Blueprints/BP_Character.CanPlayer1NotMove` false _characterref)
      (set `/Game/Blueprints/BP_Character.CanPlayer2NotMove` false _characterref))
    (:`else`)))

(fn `UserConstructionScript`)