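; BP_dancers is a moving dancers obstacle that circles a target actor and makes BP_Character drop its Table and Pot on contact.
; Tick accumulates angle from RotationSpeed and Clockwise, places the actor on a radius via RotateActoraroundPoint, and yaws Dancers1.
; Box overlap sets the character's LetTableFall flag and enables physics and gravity on both props.
; The nodes that would snap Box to Dancers1 are disconnected.
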(event `self.ReceiveTick`
  (params (DeltaSeconds :type "Float (single-precision)"))
  (bind _returnvalue (* DeltaSeconds (`self.RotationSpeed`)))
  (bind _output_get (set `self.CurrentRotation` (+ (`self.CurrentRotation`) (* _returnvalue (`KismetMathLibrary.SelectFloat` 1.0 -1.0 (`self.Clockwise`))))))
  (`self.RotateActoraroundPoint` self (`self.TargetActor`) (`SceneComponent.K2_GetComponentLocation` (`self.dancers__1_`)) (`self.Radius`) (`self.StartingAngle`) _output_get)
  (if (`self.Clockwise`)
    (bind _output_get_2 (set `self.CurrentZRotation` (- (`self.CurrentZRotation`) _returnvalue)))
    (`SceneComponent.K2_SetWorldRotation` (`self.dancers__1_`) (`KismetMathLibrary.MakeRotator` 0.0 0.0 _output_get_2) false false)
    (else
      (bind _output_get_3 (set `self.CurrentZRotation` (+ (`self.CurrentZRotation`) _returnvalue)))
      (`SceneComponent.K2_SetWorldRotation` (`self.dancers__1_`) (`KismetMathLibrary.MakeRotator` 0.0 0.0 _output_get_3) false false))))

(event `self.Box.OnComponentBeginOverlap`
  (params (OverlappedComponent :type "PrimitiveComponent Object Reference") (OtherActor :type "Actor Object Reference") (OtherComp :type "PrimitiveComponent Object Reference") (OtherBodyIndex :type Integer) (bFromSweep :type Boolean) (SweepResult :type "HitResult Structure (by ref)"))
  (bind _asbp_character (cast `/Game/Blueprints/BP_Character` OtherActor))
  (set `/Game/Blueprints/BP_Character.LetTableFall` true _asbp_character)
  (bind _table (`/Game/Blueprints/BP_Character.Table` _asbp_character))
  (`PrimitiveComponent.SetSimulatePhysics` _table true)
  (`PrimitiveComponent.SetEnableGravity` _table true)
  (bind _pot (`/Game/Blueprints/BP_Character.Pot` _asbp_character))
  (`PrimitiveComponent.SetSimulatePhysics` _pot true)
  (`PrimitiveComponent.SetEnableGravity` _pot true))

(fn `RotateActoraroundPoint`
  (params (ActorToRotate :type "Actor Object Reference") (TargetActor :type "Actor Object Reference") (TargetLocation :type "Vector Structure") (Radius :type "Float (double-precision)") (Angle :type "Float (double-precision)") (RotationRate :type "Float (double-precision)"))
  (locals (LActorToRotate :type "Actor Object Reference") (LTargetActor :type "Actor Object Reference") (LLocation :type "Vector Structure") (LRadius :type "Float (double-precision)") (LAngle :type "Float (double-precision)") (LRotateRate :type "Float (double-precision)"))
  (set `local.LActorToRotate` ActorToRotate)
  (set `local.LTargetActor` TargetActor)
  (set `local.LLocation` TargetLocation)
  (set `local.LRadius` Radius)
  (set `local.LAngle` Angle)
  (set `local.LRotateRate` RotationRate)
  (`/Engine/EditorBlueprintResources/StandardMacros.IsValid` (`local.LTargetActor`)
    (:`Is Valid`
      (set `local.LLocation` (`self.K2_GetActorLocation` (`local.LTargetActor`))))
    (:`Is Not Valid`
      _))
  (`self.K2_SetActorLocation` (`local.LActorToRotate`) (+ (`local.LLocation`) (`KismetMathLibrary.RotateAngleAxis` (`KismetMathLibrary.MakeVector` (`local.LRadius`)) (+ (`local.LRotateRate`) (`local.LAngle`)) (0.0 0.0 1.0))) false false)
  (return))

(fn `UserConstructionScript`)