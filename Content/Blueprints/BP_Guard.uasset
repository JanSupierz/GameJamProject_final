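; Patrolling guard that walks between two targets and makes the player's table and pot fall when BP_Character enters its ViewBox.
; Tick moves the mesh back and forth, waiting at each end while it turns at a speed derived from the wait time.
; Tick also pauses or resumes a 2D guard sound by the player camera socket's Y distance, using separate play and mute ranges.
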(event `self.ReceiveBeginPlay`
  (bind _returnvalue (`GameplayStatics.SpawnSound2D` "/Game/audio/Guards_Cue.Guards_Cue" 1.0 1.0 0.0 null))
  (bind _output_get (set `self.Sound` _returnvalue))
  (`AudioComponent.SetPaused` _output_get true)
  (`AudioComponent.SetVolumeMultiplier` _output_get 5.0)
  (set `self.TurnSpeed` (/ 180.0 (`self.WaitTime`))))

(event `self.ReceiveTick`
  (params (DeltaSeconds :type "Float (single-precision)"))
  (bind _mesh (`self.Mesh`))
  (bind _returnvalue_x (`KismetMathLibrary.BreakVector` (`SceneComponent.K2_GetComponentLocation` (`self.Mesh`))))
  (bind _returnvalue_x_2 (`KismetMathLibrary.BreakVector` (`SceneComponent.K2_GetComponentLocation` (`self.Target2`))))
  (bind _returnvalue_x_3 (`KismetMathLibrary.BreakVector` (`SceneComponent.K2_GetComponentLocation` (`self.Mesh`))))
  (bind (_returnvalue_x_4 _returnvalue_y) (`KismetMathLibrary.BreakVector` (`SceneComponent.K2_GetComponentLocation` (`self.Mesh`))))
  (bind _returnvalue_x_5 (`KismetMathLibrary.BreakVector` (`SceneComponent.K2_GetComponentLocation` (`self.Target1`))))
  (`|ExecutionSequence`
    (:`then_0`
      (if (`self.StartWalking`)
        (if (`self.IsMovingRight`)
          (`SceneComponent.K2_SetRelativeRotation` _mesh (struct :`Yaw` -90.0) false false)
          (`SceneComponent.K2_AddLocalOffset` (`self.Mesh`) (`KismetMathLibrary.MakeVector` 0.0 (* DeltaSeconds (`self.MoveSpeed`))) false false)
          (if (>= _returnvalue_x_3 _returnvalue_x_2)
            (set `self.IsMovingRight` false)
            (set `self.StartWalking` false)
            (`KismetSystemLibrary.Delay` (`self.WaitTime`))
            (set `self.StartWalking` true))
          (else
            (`SceneComponent.K2_SetRelativeRotation` _mesh (struct :`Yaw` 90.0) false false)
            (`SceneComponent.K2_AddLocalOffset` (`self.Mesh`) (`KismetMathLibrary.MakeVector` 0.0 (* DeltaSeconds (`self.MoveSpeed`))) false false)
            (if (<= _returnvalue_x _returnvalue_x_5)
              (set `self.IsMovingRight` true)
              (set `self.StartWalking` false)
              (`KismetSystemLibrary.Delay` (`self.WaitTime`))
              (set `self.StartWalking` true))))
        (else
          (`SceneComponent.K2_AddRelativeRotation` (`self.Mesh`) (`KismetMathLibrary.MakeRotator` 0.0 0.0 (* DeltaSeconds (`self.TurnSpeed`))) false false))))
    (:`then_1`
      (bind _asbp_character (cast `/Game/Blueprints/BP_Character` (`GameplayStatics.GetPlayerPawn` 0)))
      (if (`self.IsPaused`)
        (bind (_returnvalue_x_6 _returnvalue_y_2) (`KismetMathLibrary.BreakVector` (`SceneComponent.K2_GetComponentLocation` (`/Game/Blueprints/BP_Character.CameraSocket` _asbp_character))))
        (bind _returnvalue (`KismetMathLibrary.Abs` (- _returnvalue_y_2 _returnvalue_y)))
        (if (< _returnvalue (`self.PlayRange`))
          (`AudioComponent.SetPaused` (`self.Sound`) false)
          (set `self.IsPaused` false))
        (elif (> _returnvalue (`self.MuteRange`))
          (`AudioComponent.SetPaused` (`self.Sound`) true)
          (set `self.IsPaused` true))))))

(event `self.ViewBox.OnComponentBeginOverlap`
  (params (OverlappedComponent :type "PrimitiveComponent Object Reference") (OtherActor :type "Actor Object Reference") (OtherComp :type "PrimitiveComponent Object Reference") (OtherBodyIndex :type Integer) (bFromSweep :type Boolean) (SweepResult :type "HitResult Structure (by ref)"))
  (bind _asbp_character (cast `/Game/Blueprints/BP_Character` OtherActor))
  (set `/Game/Blueprints/BP_Character.LetTableFall` true _asbp_character)
  (bind _table (`/Game/Blueprints/BP_Character.Table` _asbp_character))
  (`PrimitiveComponent.SetSimulatePhysics` _table true)
  (`PrimitiveComponent.SetEnableGravity` _table true)
  (bind _pot (`/Game/Blueprints/BP_Character.Pot` _asbp_character))
  (`PrimitiveComponent.SetSimulatePhysics` _pot true)
  (`PrimitiveComponent.SetEnableGravity` _pot true))

(fn `UserConstructionScript`)