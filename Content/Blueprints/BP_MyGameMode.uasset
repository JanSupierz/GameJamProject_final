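; Game mode that runs a countdown timer and manages the HUD, game-over screen and level restart.
; Once HasGameStarted is true, Tick decrements AmountOfTimeLeft by delta time and creates the HUD widget a single time.
; GameOverEvent plays a breaking-teapot sound and shows the end screen once, but nothing in this graph calls it.
; RestartGame reopens the current level by name.
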(event `self.ReceiveBeginPlay`)

(event `self.ReceiveTick`
  (params (DeltaSeconds :type "Float (single-precision)"))
  (if (`self.hasGameStarted`)
    (set `self.AmountOfTimeLeft` (- (`self.AmountOfTimeLeft`) DeltaSeconds))
    (`/Engine/EditorBlueprintResources/StandardMacros.DoOnce` false
      (:`Completed`
        (bind _returnvalue (`|CreateWidget` "/Game/Blueprints/BP_HUD.BP_HUD_C" (`GameplayStatics.GetPlayerController` 0)))
        (`UserWidget.AddToViewport` _returnvalue 0)))))

(event `GameOverEvent`
  (`/Engine/EditorBlueprintResources/StandardMacros.DoOnce` false
    (:`Completed`
      (`GameplayStatics.PlaySound2D` "/Game/audio/BreakingTeapot.BreakingTeapot" 1.0 1.0 0.0 null null)
      (bind _returnvalue (`|CreateWidget` "/Game/Blueprints/BP_EndScreen.BP_EndScreen_C" (`GameplayStatics.GetPlayerController` 0)))
      (`UserWidget.AddToViewport` _returnvalue 0))))

(event `RestartGame`
  (bind _returnvalue (`GameplayStatics.GetCurrentLevelName` true))
  (`GameplayStatics.OpenLevel` (`KismetStringLibrary.Conv_StringToName` _returnvalue)))

(fn `UserConstructionScript`)