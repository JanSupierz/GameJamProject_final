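; BP_FallingStatue is a statue that topples once when a BP_Character enters its trigger, playing a 2D sound.
; Tick then tips the mesh with swept local roll rotation at FallSpeed, up to a fixed roll limit.
; Tick also keeps physics off while world roll is near zero or below, then enables it once tilted, constrained to the XZ plane.
; An EndRotation lerp variant is left unconnected.
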(event `self.ReceiveBeginPlay`)

(event `self.trigger.OnComponentBeginOverlap`
  (params (OverlappedComponent :type "PrimitiveComponent Object Reference") (OtherActor :type "Actor Object Reference") (OtherComp :type "PrimitiveComponent Object Reference") (OtherBodyIndex :type Integer) (bFromSweep :type Boolean) (SweepResult :type "HitResult Structure (by ref)"))
  (cast `/Game/Blueprints/BP_Character` OtherActor)
  (if (not (`self.fall`))
    (`GameplayStatics.PlaySound2D` "/Game/audio/FallingStatue.FallingStatue" 1.0 1.0 0.0 null null)
    (set `self.fall` true)
    (`PrimitiveComponent.SetSimulatePhysics` (`self.mesh`) true)))

(event `self.ReceiveTick`
  (params (DeltaSeconds :type "Float (single-precision)"))
  (bind _mesh (`self.mesh`))
  (bind _returnvalue_roll (`KismetMathLibrary.BreakRotator` (`SceneComponent.K2_GetComponentRotation` (`self.mesh`))))
  (bind _relativerotation_roll (`KismetMathLibrary.BreakRotator` (`SceneComponent.RelativeRotation` _mesh)))
  (`|ExecutionSequence`
    (:`then_0`
      (if (and (`self.fall`) (> 50.0 _relativerotation_roll))
        (`SceneComponent.K2_AddLocalRotation` _mesh (`KismetMathLibrary.MakeRotator` (* DeltaSeconds (`self.fallSpeed`))) true false)))
    (:`then_1`
      (if (<= _returnvalue_roll 0.001)
        (`PrimitiveComponent.SetSimulatePhysics` (`self.mesh`) false)
        (elif (not (`self.onGround`))
          (`PrimitiveComponent.SetSimulatePhysics` (`self.mesh`) true)
          (set `self.onGround` true)
          (`PrimitiveComponent.SetConstraintMode` (`self.mesh`) "XZPlane"))))))

(fn `UserConstructionScript`)