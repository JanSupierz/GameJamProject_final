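; BP_MovingChair is a moving chair obstacle that makes the player character's table and pot fall on contact.
; Tick slides the static mesh horizontally at Speed toward CurrentTarget, ping-ponging between two billboard components used as waypoints.
; When BP_Character overlaps Deadbox, it sets that character's LetTableFall flag and enables physics and gravity on its Table and Pot.
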(event `self.ReceiveBeginPlay`
  (set `self.currentTarget` (`self.Billboard`)))

(event `self.ReceiveTick`
  (params (DeltaSeconds :type "Float (single-precision)"))
  (bind _staticmesh (`self.StaticMesh`))
  (bind _billboard (`self.Billboard`))
  (bind _returnvalue (`SceneComponent.K2_GetComponentLocation` _staticmesh))
  (bind (_returnvalue_x _returnvalue_y) (`KismetMathLibrary.BreakVector` (- (`SceneComponent.K2_GetComponentLocation` (`self.currentTarget`)) _returnvalue)))
  (bind _returnvalue_2 (`KismetMathLibrary.MakeVector` _returnvalue_x _returnvalue_y))
  (`SceneComponent.K2_SetWorldLocation` _staticmesh (+ _returnvalue (* (`KismetMathLibrary.Normal` _returnvalue_2) (`self.speed`) DeltaSeconds)) false false)
  (if (< (`KismetMathLibrary.VSize` _returnvalue_2) 5.0)
    (if (== (`self.currentTarget`) _billboard)
      (set `self.currentTarget` (`self.Billboard1`))
      (else
        (set `self.currentTarget` _billboard)))))

(event `self.Deadbox.OnComponentBeginOverlap`
  (params (OverlappedComponent :type "PrimitiveComponent Object Reference") (OtherActor :type "Actor Object Reference") (OtherComp :type "PrimitiveComponent Object Reference") (OtherBodyIndex :type Integer) (bFromSweep :type Boolean) (SweepResult :type "HitResult Structure (by ref)"))
  (bind _asbp_character (cast `/Game/Blueprints/BP_Character` OtherActor))
  (set `/Game/Blueprints/BP_Character.LetTableFall` true _asbp_character)
  (bind _table (`/Game/Blueprints/BP_Character.Table` _asbp_character))
  (`PrimitiveComponent.SetSimulatePhysics` _table true)
  (`PrimitiveComponent.SetEnableGravity` _table true)
  (bind _pot (`/Game/Blueprints/BP_Character.Pot` _asbp_character))
  (`PrimitiveComponent.SetSimulatePhysics` _pot true)
  (`PrimitiveComponent.SetEnableGravity` _pot true))

(fn `UserConstructionScript`)