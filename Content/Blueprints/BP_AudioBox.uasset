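; BP_AudioBox is an actor that plays a sound at its root location while a BP_Character is inside its box.
; Each Tick it polls the Box's overlapping actors instead of using overlap events, with a DoOnce limiting the spawn to one audio component per stay.
; When no character overlaps, it stops and destroys that component and resets the DoOnce for the next entry.
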(event `self.ReceiveTick`
  (params (DeltaSeconds :type "Float (single-precision)"))
  (if (> (`KismetArrayLibrary.Array_Length` (`PrimitiveComponent.GetOverlappingActors` (`self.Box`) "/Game/Blueprints/BP_Character.BP_Character_C")) 0)
    (`/Engine/EditorBlueprintResources/StandardMacros.DoOnce` false :!label _label
      (:`Completed`
        (bind _returnvalue (`GameplayStatics.SpawnSoundAtLocation` (`self.sound`) (`SceneComponent.K2_GetComponentLocation` (`self.DefaultSceneRoot`)) (struct) 1.0 1.0 0.0 null null))
        (set `self.AudioComp` _returnvalue)))
    (else
      (bind _audiocomp (`self.AudioComp`)
        (:`then`
          (`AudioComponent.Stop` _audiocomp)
          (`ActorComponent.K2_DestroyComponent` _audiocomp)
          (goto _label :!via `Reset`))
        (:`else`
          (goto _label :!via `Reset`))))))

(fn `UserConstructionScript`)